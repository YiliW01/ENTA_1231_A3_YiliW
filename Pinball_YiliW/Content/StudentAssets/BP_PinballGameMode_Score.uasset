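; Pinball game mode that handles scoring, ball count and game over.
; State lives in BP_PinballGameState: BeginPlay sets the starting balls directly, and AddScore adds points through SetScore.
; OnBallLost decrements the count through SetBalls, then calls SpawnBall while balls remain or adds GameOverWidget to the viewport.
; Each event casts the game state and stops if the cast fails.
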(event `/Game/StudentAssets/BPI_ScoreReceiver.AddScore`
  (params (Points :type "Float (double-precision)"))
  (bind _asbp_pinball_game_state (cast `/Game/StudentAssets/BP_PinballGameState` (`GameplayStatics.GetGameState`)))
  (`/Game/StudentAssets/BP_PinballGameState.SetScore` _asbp_pinball_game_state (+ (`/Game/StudentAssets/BP_PinballGameState.Score` _asbp_pinball_game_state) Points)))

(event `self.OnBallLost`
  (bind _asbp_pinball_game_state (cast `/Game/StudentAssets/BP_PinballGameState` (`GameplayStatics.GetGameState`)))
  (bind _ballsremaining (`/Game/StudentAssets/BP_PinballGameState.BallsRemaining` _asbp_pinball_game_state))
  (bind _result (`/Engine/EditorBlueprintResources/StandardMacros.DecrementInt` _ballsremaining)
    (:`  `
      (`/Game/StudentAssets/BP_PinballGameState.SetBalls` _asbp_pinball_game_state _result)
      (if (> _ballsremaining 0)
        (`self.SpawnBall`)
        (else
          (`UserWidget.AddToViewport` (`self.GameOverWidget`) 0))))))

(event `self.ReceiveBeginPlay`
  (bind _asbp_pinball_game_state (cast `/Game/StudentAssets/BP_PinballGameState` (`GameplayStatics.GetGameState`)))
  (set `/Game/StudentAssets/BP_PinballGameState.BallsRemaining` 3 _asbp_pinball_game_state))

(fn `UserConstructionScript`
  (`parent.UserConstructionScript`))