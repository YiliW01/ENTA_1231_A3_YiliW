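; BP_Bumper is a pinball bumper that knocks reactive objects away and awards score.
; On capsule overlap, it casts the other actor to BPI_PinballReactive and sends an impulse of MaxForce pointing from the bumper toward the overlapping component.
; It then passes ScoreValue to the game mode through AddScoreMessage; actors failing the cast get neither impulse nor score.
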(event `self.Capsule.OnComponentBeginOverlap`
  (params (OverlappedComponent :type "PrimitiveComponent Object Reference") (OtherActor :type "Actor Object Reference") (OtherComp :type "PrimitiveComponent Object Reference") (OtherBodyIndex :type Integer) (bFromSweep :type Boolean) (SweepResult :type "HitResult Structure (by ref)"))
  (bind _asbpi_pinball_reactive (cast `/Game/StudentAssets/BPI_PinballReactive` OtherActor))
  (`/Game/StudentAssets/BPI_PinballReactive.PinballImpulseEvent` _asbpi_pinball_reactive (* (`self.MaxForce`) (`KismetMathLibrary.Normal` (- (`SceneComponent.K2_GetComponentLocation` OtherComp) (`self.K2_GetActorLocation`)))))
  (message `/Game/StudentAssets/BPI_ScoreReceiver.AddScore` (`GameplayStatics.GetGameMode`) (`self.ScoreValue`)))

(fn `UserConstructionScript`)