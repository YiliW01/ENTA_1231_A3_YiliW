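; BP_PinballGameState is a game state Blueprint that holds the score and remaining ball count for a pinball game.
; SetScore and SetBalls store the new value, then broadcast it through the OnScoreChanged and OnBallsChanged event dispatchers.
; BeginPlay is empty, and a disconnected test chain in the event graph that sets and prints both values never runs.
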(event `self.ReceiveBeginPlay`)

(fn `SetBalls`
  (params (NewBalls :type Integer))
  (bind _output_get (set `self.BallsRemaining` NewBalls))
  (`self.OnBallsChanged` _output_get))

(fn `SetScore`
  (params (NewScore :type "Float (double-precision)"))
  (bind _output_get (set `self.Score` NewScore))
  (`self.OnScoreChanged` _output_get))

(fn `UserConstructionScript`)